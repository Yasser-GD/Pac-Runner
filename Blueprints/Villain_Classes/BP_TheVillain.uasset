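; BP_TheVillain is the ghost-like enemy pawn in a Pac-Man-style game, flagging the player killed on kill-box overlap unless CantKillPlayer is set.
; It loops an attached howling wind sound and takes movement speed changes through a dispatcher.
; Player events temporarily swap in a vulnerable material or stop the wind when a ghost dies.
; UpdateMovementTarget chases the player via AI MoveTo; random reach-point logic is unconnected.
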(event `self.ReceiveBeginPlay`
  (bind _returnvalue (`GameplayStatics.SpawnSoundAttached` "/Game/Sounds/Howling_Wind_Sound/Howling_Wind_SoundCue.Howling_Wind_SoundCue" (`self.TheViliain`) "None" (0.0 0.0 0.0) (struct) "KeepRelativeOffset" false 1.0 1.0 0.0 "/Game/Sounds/Howling_Wind_Sound/Howling_Wind_Attenuation.Howling_Wind_Attenuation" null false))
  (bind _output_get (set `self.Howling Wind Sound Component ` _returnvalue))
  (add `AudioComponent.OnAudioFinished` _output_get (delegate `OnAudioFinished_Event_0`))
  (bind _aspacman_char (cast `Pacman_Char` (`GameplayStatics.GetPlayerPawn` 0)))
  (set `self.As Pacman Char` _aspacman_char)
  (add `self.ChangeSpeedCast` (delegate `ChangeSpeedCast_Event`))
  (add `Pacman_Char.BeTheEaterEvent` (`self.As Pacman Char`) (delegate `BeTheEaterEvent_Event_0`))
  (add `Pacman_Char.KilledGhostEvent` (`self.As Pacman Char`) (delegate `KilledGhostEvent_Event_0`)))

(event `OnAudioFinished_Event_0`
  (`AudioComponent.Play` (`self.Howling Wind Sound Component `) 0.0))

(event `ChangeSpeedCast_Event` :!signature `self.ChangeSpeedCast`
  (params (NewSpeed :type "Float (single-precision)"))
  (set `FloatingPawnMovement.MaxSpeed` NewSpeed (`self.FloatingPawnMovement`)))

(event `KilledGhostEvent_Event_0`
  (params (AIController :type "Controller Object Reference"))
  (`AudioComponent.Stop` (`self.Howling Wind Sound Component `)))

(event `BeTheEaterEvent_Event_0`
  (params (EndTime :type Integer))
  (`PrimitiveComponent.SetMaterial` (`self.TheViliain`) 2 "/Game/Blueprints/End_Game_Mode_Classes/Ghosts_Stuff/Materials/Got_Hit_Materials/M_EnemyVulnerable2.M_EnemyVulnerable2")
  (`KismetSystemLibrary.Delay` (`KismetMathLibrary.Conv_IntToDouble` EndTime))
  (`PrimitiveComponent.SetMaterial` (`self.TheViliain`) 2 "/Game/Blueprints/End_Game_Mode_Classes/Ghosts_Stuff/Materials/Got_Hit_Materials/M_EnemyPawnRed.M_EnemyPawnRed"))

(event `self.ReceiveTick`
  (params (DeltaSeconds :type "Float (single-precision)")))

(event `self.Kill Player Box.OnComponentBeginOverlap`
  (params (OverlappedComponent :type "PrimitiveComponent Object Reference") (OtherActor :type "Actor Object Reference") (OtherComp :type "PrimitiveComponent Object Reference") (OtherBodyIndex :type Integer) (bFromSweep :type Boolean) (SweepResult :type "HitResult Structure (by ref)"))
  (bind _asbp_pacman_char (cast `/Game/Blueprints/BP_Pacman_Char` OtherActor))
  (if (not (`self.CantKillPlayer`))
    (set `Pacman_Char.PlayerKilled` true _asbp_pacman_char)
    (`StaticMeshComponent.SetStaticMesh` (`self.TheViliain`) "/Game/Pacman/Meshes/SM_Enemy_Vulnerable.SM_Enemy_Vulnerable")))

(fn `UpdateMovementTarget`
  (locals (`AI Controllerrrr` :type "AIController Object Reference"))
  (set `local.AI Controllerrrr` (`AIBlueprintHelperLibrary.GetAIController` (`self.GetController`)))
  (`AIController.MoveToActor` (`local.AI Controllerrrr`) (`GameplayStatics.GetPlayerPawn` 0) 0.0 false true true null true))

(fn `UserConstructionScript`)