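; BP_Pacman_Char is the Pac-Man player character, handling timed abilities, death and menu input.
; BeginPlay binds the Guide Foodie and Be The Eater events, which show GuidePlane or PlayerEaterBox for a delay, then clear the in-use flags.
; Tick polls PlayerKilled to show the dying widget once.
; Escape opens the pause widget without pausing the game, F6 takes a screenshot, and save-delete logic is unwired.
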(event `BeTheEaterEvent_Event_0` :!signature `self.BeTheEaterEvent`
  (params (EndTime :type Integer))
  (`SceneComponent.SetVisibility` (`self.PlayerEaterBox`) true false)
  (`KismetSystemLibrary.Delay` (`KismetMathLibrary.Conv_IntToDouble` (`self.Eater_EventEndTimer`)))
  (`SceneComponent.SetVisibility` (`self.PlayerEaterBox`) false false)
  (set `self.BeTheEaterOnUse` false)
  (set `self.OnUseAnyAbility` false))

(event `self.ReceiveBeginPlay`
  (add `self.GuideFoodieEvent` (delegate `GuideFoodieEvent_Event_0`))
  (add `self.BeTheEaterEvent` (delegate `BeTheEaterEvent_Event_0`)))

(event `GuideFoodieEvent_Event_0`
  (`SceneComponent.SetVisibility` (`self.Guide Plane`) true false)
  (`KismetSystemLibrary.Delay` (`self.Guide Foodiee End Time`))
  (`SceneComponent.SetVisibility` (`self.Guide Plane`) false false)
  (set `self.GuideAbilityOnUse` false)
  (set `self.OnUseAnyAbility` false))

(event `self.ReceiveTick`
  (params (DeltaSeconds :type "Float (single-precision)"))
  (if (`self.Is Already Dead `)
    _
    (elif (`self.PlayerKilled`)
      (bind _returnvalue (`|CreateWidget` "/Game/Blueprints/Widgets_/Dying_Widget.Dying_Widget_C"))
      (`UserWidget.AddToViewport` _returnvalue 0)
      (set `PlayerController.bShowMouseCursor` true (`GameplayStatics.GetPlayerController` 0))
      (set `self.Is Already Dead ` true))))

(event `Key|F6`
  (params (Key :type "Key Structure"))
  (:`Pressed`
    (`KismetSystemLibrary.PrintString` "Screenshot Taken ")
    (`KismetSystemLibrary.Delay` 1.0)
    (`KismetSystemLibrary.ExecuteConsoleCommand` "HighResShot 2" null)))

(event `Key|P`
  (params (Key :type "Key Structure")))

(event `Key|Escape`
  (params (Key :type "Key Structure"))
  (bind _returnvalue (`GameplayStatics.GetPlayerController` 0))
  (:`Pressed`
    (bind _returnvalue_2 (`|CreateWidget` "/Game/Blueprints/Widgets_/UI/Pause_Widget.Pause_Widget_C"))
    (`UserWidget.AddToViewport` _returnvalue_2 0)
    (`GameplayStatics.SetGamePaused` false)
    (`WidgetBlueprintLibrary.SetInputMode_UIOnlyEx` _returnvalue null)
    (set `PlayerController.bShowMouseCursor` true _returnvalue)))

(fn `UserConstructionScript`)