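; Main menu pawn that sets up level unlock progress from a save slot when play begins.
; If the "Save1" slot exists, it loads the SaveGame_1 and copies its three level flags into Pacman_GameInstance.
; Otherwise it creates a new save with only the first level enabled, mirrors that flag to the game instance and writes the slot.
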(event `self.ReceiveBeginPlay`
  (bind _as_pacman_game_instance (`self.As Pacman Game Instance`))
  (bind _aspacman_game_instance (cast `Pacman_GameInstance` (`GameplayStatics.GetGameInstance`)))
  (set `self.As Pacman Game Instance` _aspacman_game_instance)
  (bind _returnvalue (`GameplayStatics.DoesSaveGameExist` "Save1"))
  (if _returnvalue
    (bind _returnvalue_2 (`GameplayStatics.LoadGameFromSlot` "Save1"))
    (bind _assave_game_1 (cast `/Game/Blueprints/Save_Game/SaveGame_1` _returnvalue_2))
    (set `self.BP_Save1` _assave_game_1)
    (set `Pacman_GameInstance.Level_One` (`/Game/Blueprints/Save_Game/SaveGame_1.Level 1` _assave_game_1) _as_pacman_game_instance)
    (set `Pacman_GameInstance.Level_Two` (`/Game/Blueprints/Save_Game/SaveGame_1.Level 2` _assave_game_1) _as_pacman_game_instance)
    (set `Pacman_GameInstance.Level_Three` (`/Game/Blueprints/Save_Game/SaveGame_1.Level 3` _assave_game_1) _as_pacman_game_instance)
    (`KismetSystemLibrary.PrintString` "SAve Game Exsists" true true (struct :`R` 0.997405 :`G` 0.099455 :`B` 1.0 :`A` 1.0) 10.0)
    (else
      (bind _returnvalue_3 (`GameplayStatics.CreateSaveGameObject` "/Game/Blueprints/Save_Game/SaveGame_1.SaveGame_1_C"))
      (bind _output_get (set `/Game/Blueprints/Save_Game/SaveGame_1.Level 1` true _returnvalue_3))
      (set `Pacman_GameInstance.Level_One` _output_get (`self.As Pacman Game Instance`))
      (`GameplayStatics.SaveGameToSlot` _returnvalue_3 "Save1")
      (set `self.BP_Save1` _returnvalue_3))))

(fn `UserConstructionScript`)